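; Flipper actor that swings its flipper component between a rest and a flipped rotation, configurable as a left or right unit.
; The construction script derives both rotations from FlipType, applies the rest pose and mirrors the component on X for the right side.
; Flip and Flop events, with no caller in this Blueprint, use MoveComponentTo to rotate to either pose over FlipTime.
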(event `self.ReceiveBeginPlay`)

(event `Flip`
  (`KismetSystemLibrary.MoveComponentTo` (`self.Fipper`) (0.0 0.0 0.0) (`self.EndRotation`) false false (`self.FlipTime`)))

(event `Flop`
  (`KismetSystemLibrary.MoveComponentTo` (`self.Fipper`) (0.0 0.0 0.0) (`self.StartRotation`) false false (`self.FlipTime`)))

(fn `UserConstructionScript`
  (set `self.StartRotation` (select `/Game/Blueprints/FlipType` (`self.FlipType`) :`NewEnumerator0` (struct :`Yaw` 20.0) :`NewEnumerator1` (struct :`Yaw` -20.0) :!type "Rotator Structure"))
  (set `self.EndRotation` (select `/Game/Blueprints/FlipType` (`self.FlipType`) :`NewEnumerator0` (struct :`Yaw` -20.0) :`NewEnumerator1` (struct :`Yaw` 20.0) :!type "Rotator Structure"))
  (`SceneComponent.K2_SetRelativeRotation` (`self.Fipper`) (`self.StartRotation`) false false)
  (switch `/Game/Blueprints/FlipType` (`self.FlipType`)
    (:`NewEnumerator1`
      (`SceneComponent.SetRelativeScale3D` (`self.Fipper`) (-1.0 1.0 1.0)))))